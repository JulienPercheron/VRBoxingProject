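; Carlos is the AI boxing opponent in a VR boxing game, tracking life points and reporting a knockout when they run out.
; SetState pushes his current action to the CarlosAnimations AnimBP.
; Glove overlaps on head or body trigger the matching hit state and remove a life point.
; Tick randomly starts a punch while the VR pawn is inside PunchTrigger, which also toggles CanTakeHit, though hits never check it here.
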(event `Iddle`
  (`self.SetState` "NewEnumerator0")
  (set `self.canTakeHit` true))

(event `IsPunching`
  (`self.SetState` "NewEnumerator1"))

(event `Takes a hit`
  (params (`Carlos State` :type "/Game/VRBoxing/Model/AnimationsBox/Animations/CarlosStates Enum" :default "NewEnumerator0"))
  (`self.SetState` `Carlos State`)
  (bind _result (`/Engine/EditorBlueprintResources/StandardMacros.DecrementFloat` (`KismetMathLibrary.Conv_IntToDouble` (`self.Life points`)))
    (:`  `
      (set `self.Life points` (`KismetMathLibrary.FTrunc` _result)))))

(event `self.CarlosHead.OnComponentBeginOverlap`
  (params (OverlappedComponent :type "PrimitiveComponent Object Reference") (OtherActor :type "Actor Object Reference") (OtherComp :type "PrimitiveComponent Object Reference") (OtherBodyIndex :type Integer) (bFromSweep :type Boolean) (SweepResult :type "HitResult Structure (by ref)"))
  (cast `/Game/VRBoxing/Blueprints/LBoxingGloves` OtherActor
    (:`then`
      _)
    (:`CastFailed`
      (cast `/Game/VRBoxing/Blueprints/RBoxingGloves` OtherActor)))
  (`self.Takes a hit` "NewEnumerator5"))

(event `self.CarlosBody.OnComponentBeginOverlap`
  (params (OverlappedComponent :type "PrimitiveComponent Object Reference") (OtherActor :type "Actor Object Reference") (OtherComp :type "PrimitiveComponent Object Reference") (OtherBodyIndex :type Integer) (bFromSweep :type Boolean) (SweepResult :type "HitResult Structure (by ref)"))
  (cast `/Game/VRBoxing/Blueprints/LBoxingGloves` OtherActor
    (:`then`
      _)
    (:`CastFailed`
      (cast `/Game/VRBoxing/Blueprints/RBoxingGloves` OtherActor)))
  (`self.Takes a hit` "NewEnumerator2"))

(event `self.ReceiveTick`
  (params (DeltaSeconds :type "Float (single-precision)"))
  (if (and (== (`KismetMathLibrary.RandomIntegerInRange` 0 50) 1) (`self.playerInRange`) (`|EnumInequality` (`self.SelectedAction`) "NewEnumerator1"))
    (`self.SetState` "NewEnumerator1")))

(event `self.PunchTrigger.OnComponentBeginOverlap`
  (params (OverlappedComponent :type "PrimitiveComponent Object Reference") (OtherActor :type "Actor Object Reference") (OtherComp :type "PrimitiveComponent Object Reference") (OtherBodyIndex :type Integer) (bFromSweep :type Boolean) (SweepResult :type "HitResult Structure (by ref)"))
  (cast `/Game/VRTemplate/Blueprints/VRPawn` OtherActor)
  (set `self.playerInRange` true)
  (set `self.canTakeHit` true))

(event `self.PunchTrigger.OnComponentEndOverlap`
  (params (OverlappedComponent :type "PrimitiveComponent Object Reference") (OtherActor :type "Actor Object Reference") (OtherComp :type "PrimitiveComponent Object Reference") (OtherBodyIndex :type Integer))
  (cast `/Game/VRTemplate/Blueprints/VRPawn` OtherActor)
  (set `self.playerInRange` false)
  (set `self.canTakeHit` false))

(fn `IsKo`
  (returns (isKo :type Boolean))
  (return (<= (`self.Life points`) 0)))

(fn `SetState`
  (params (CarlosState :type "/Game/VRBoxing/Model/AnimationsBox/Animations/CarlosStates Enum" :default "NewEnumerator0"))
  (set `self.SelectedAction` CarlosState)
  (bind _ascarlos_animations (cast `/Game/VRBoxing/Model/AnimationsBox/Animations/CarlosAnimations` (`SkeletalMeshComponent.GetAnimInstance` (`self.CarlosSkeletal`))))
  (set `/Game/VRBoxing/Model/AnimationsBox/Animations/CarlosAnimations.CarlosState` (`self.SelectedAction`) _ascarlos_animations))

(fn `UserConstructionScript`)