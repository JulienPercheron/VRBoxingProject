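; RBoxingGloves is a VR boxing glove actor that detects when a block starts and ends.
; Its BlockingTrigger reacts to overlaps with box components tagged LHand or RHand, setting Blocked on begin and clearing it on end.
; Each change also calls Blocking or Unblock on player 0's VRPawn, with no overlap counting, so any matching exit ends the block.
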(event `self.BlockingTrigger.OnComponentBeginOverlap`
  (params (OverlappedComponent :type "PrimitiveComponent Object Reference") (OtherActor :type "Actor Object Reference") (OtherComp :type "PrimitiveComponent Object Reference") (OtherBodyIndex :type Integer) (bFromSweep :type Boolean) (SweepResult :type "HitResult Structure (by ref)"))
  (bind _asbox_collision (cast `BoxComponent` OtherComp))
  (if (or (`ActorComponent.ComponentHasTag` _asbox_collision "LHand") (`ActorComponent.ComponentHasTag` _asbox_collision "RHand"))
    (set `self.Blocked` true)
    (bind _asvrpawn (cast `/Game/VRTemplate/Blueprints/VRPawn` (`GameplayStatics.GetPlayerPawn` 0)))
    (`/Game/VRTemplate/Blueprints/VRPawn.Blocking` _asvrpawn)))

(event `self.BlockingTrigger.OnComponentEndOverlap`
  (params (OverlappedComponent :type "PrimitiveComponent Object Reference") (OtherActor :type "Actor Object Reference") (OtherComp :type "PrimitiveComponent Object Reference") (OtherBodyIndex :type Integer))
  (bind _asbox_collision (cast `BoxComponent` OtherComp))
  (if (or (`ActorComponent.ComponentHasTag` _asbox_collision "LHand") (`ActorComponent.ComponentHasTag` _asbox_collision "RHand"))
    (set `self.Blocked` false)
    (bind _asvrpawn (cast `/Game/VRTemplate/Blueprints/VRPawn` (`GameplayStatics.GetPlayerPawn` 0)))
    (`/Game/VRTemplate/Blueprints/VRPawn.Unblock` _asvrpawn)))

(fn `UserConstructionScript`)